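; BP_Crystal is a collectable crystal that flies into the player and vanishes when the player overlaps it.
; On overlap it stores its starting location, scale and light intensity, then plays CollectionTimeline.
; The timeline's separate curves drive lerps toward the player's current location, zero scale and zero light intensity.
; The actor destroys itself when the timeline finishes.
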(event Collision|EventActorBeginOverlap
  (params (OtherActor :type Actor%20Object%20Reference))
  (Utilities|IsPlayer OtherActor
    (:isPlayer
      (CallFunction|StoreStartingValues)
      (bind (_direction _collection_progress _scale_progress _light_intensity) (Timeline|Collection%20Timeline Play) ; Smooth Lerp Alpha is the value thats changing. This creates the ease curve into how to do the lerp
        (:Update
          (CallFunction|MovetoPlayer _collection_progress)
          (CallFunction|ScaleCrystal _scale_progress)
          (CallFunction|AdjustLight _light_intensity))
        (:Finished
          (Actor|DestroyActor))))))

(fn ConstructionScript)

(fn MovetoPlayer
  (params (Alpha :type Float%20%28single-precision%29))
  (Transformation|SetActorLocation (Math|Vector|Lerp(Vector) (Variables|Default|GetstartLocation) (Transformation|GetActorLocation (Game|Player|GetPlayerPawn 0)) Alpha) false false) ; Bringing in the Alpha
)

(fn StoreStartingValues
  (Variables|Default|SetstartLocation (Transformation|GetActorLocation))
  (Variables|Default|SetstartScale (Transformation|GetActorScale3D))
  (Variables|Default|SetdefaultLightIntensity (Variables|/Script/Engine.LightComponentBase|GetIntensity (Variables|Default|GetCrystale%20Light))))

(fn ScaleCrystal
  (params (Alpha :type Float%20%28single-precision%29))
  (Transformation|SetActorScale3D (Math|Vector|Lerp(Vector) (Variables|Default|GetstartScale) "0, 0, 0" Alpha)))

(fn AdjustLight
  (params (Alpha :type Float%20%28single-precision%29))
  (Rendering|Components|Light|SetIntensity (Variables|Default|GetCrystale%20Light) (Math|Float|Lerp (Variables|Default|GetdefaultLightIntensity) 0.0 Alpha)))